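; BP_Ship is a ship Blueprint that provides mouse hover highlighting and click interaction for its turret and gun meshes.
; Hovering the turret swaps both meshes to BasicAsset01 and leaving restores DefaultMaterial, while hovering the gun swaps only the gun's material.
; Clicking either mesh calls AimingAtTarget, apparently an event dispatcher, with the aiming logic itself outside this graph.
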(event `self.TurretMeshComponent.OnBeginCursorOver`
  (params (TouchedComponent :type "PrimitiveComponent Object Reference"))
  (`PrimitiveComponent.SetMaterial` (`self.TurretMeshComponent`) 0 "/Engine/MapTemplates/Materials/BasicAsset01.BasicAsset01")
  (`PrimitiveComponent.SetMaterial` (`self.GunMeshComponent`) 0 "/Engine/MapTemplates/Materials/BasicAsset01.BasicAsset01" :!label _label))

(event `self.TurretMeshComponent.OnEndCursorOver`
  (params (TouchedComponent :type "PrimitiveComponent Object Reference"))
  (`PrimitiveComponent.SetMaterial` (`self.TurretMeshComponent`) 0 "/Engine/EngineMaterials/DefaultMaterial.DefaultMaterial")
  (`PrimitiveComponent.SetMaterial` (`self.GunMeshComponent`) 0 "/Engine/EngineMaterials/DefaultMaterial.DefaultMaterial" :!label _label_2))

(event `self.GunMeshComponent.OnBeginCursorOver`
  (params (TouchedComponent :type "PrimitiveComponent Object Reference"))
  (goto _label))

(event `self.GunMeshComponent.OnEndCursorOver`
  (params (TouchedComponent :type "PrimitiveComponent Object Reference"))
  (goto _label_2))

(event `self.TurretMeshComponent.OnClicked`
  (params (TouchedComponent :type "PrimitiveComponent Object Reference") (ButtonPressed :type "Key Structure"))
  (`self.AimingAtTarget` :!label _label_3))

(event `self.GunMeshComponent.OnClicked`
  (params (TouchedComponent :type "PrimitiveComponent Object Reference") (ButtonPressed :type "Key Structure"))
  (goto _label_3))

(fn `UserConstructionScript`)